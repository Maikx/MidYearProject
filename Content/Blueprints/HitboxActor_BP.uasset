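; HitboxActor_BP is a hitbox actor with a display component for proximity, strike and hurtbox types.
; Its SpawnHitbox event picks the display material from HitboxType, moves the display to HitboxLocation in world space, then hides it.
; The Blueprint holds no collision or damage logic, and its construction script is empty.
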(event `SpawnHitbox`
  (switch `EHitboxEnum` (`self.hitboxType`)
    (:`HB_PROXIMITY`
      (`PrimitiveComponent.SetMaterial` (`self.HitboxDisplay`) 0 "/Game/Materials/M_ProximityHitbox.M_ProximityHitbox"))
    (:`HB_STRIKE`
      (`PrimitiveComponent.SetMaterial` (`self.HitboxDisplay`) 0 "/Game/Materials/M_StrikeHitbox.M_StrikeHitbox"))
    (:`HB_HURTBOX`
      (`PrimitiveComponent.SetMaterial` (`self.HitboxDisplay`) 0 "/Game/Materials/M_HurtBox.M_HurtBox")))
  (`SceneComponent.K2_SetWorldLocation` (`self.HitboxDisplay`) (`self.hitboxLocation`) false false)
  (`SceneComponent.SetVisibility` (`self.HitboxDisplay`) false false))

(fn `UserConstructionScript`)